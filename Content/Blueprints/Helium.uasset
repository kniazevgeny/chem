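; Helium is an actor with a sphere whose glow intensifies as it nears the closest actor returned by FindClosest.
; The construction script passes the sphere and a fixed index to CustomConstruction, then stores and applies the resulting dynamic material instance.
; Every tick, it sets that material's Emission parameter inversely proportional to the distance to that closest actor.
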(event `self.ReceiveTick`
  (params (DeltaSeconds :type "Float (single-precision)"))
  (bind _closest (`self.find closest` self))
  (`MaterialInstanceDynamic.SetScalarParameterValue` (`self.MID`) "Emission" (/ 1250.0 (`self.GetDistanceTo` _closest))))

(event `self.ReceiveBeginPlay`)

(fn `NewFunction_1_0`)

(fn `UserConstructionScript`
  (bind _dynamic_material (`self.CustomConstruction` 2 (`self.Sphere`)))
  (bind _output_get (set `self.MID` _dynamic_material))
  (`PrimitiveComponent.SetMaterial` (`self.Sphere`) 0 _output_get))