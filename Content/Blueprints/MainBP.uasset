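; MainBP drives a molecule-building scene, spawning an initial object and the ButtonPlus widget on BeginPlay.
; Committed text goes unvalidated to SpawnGraphFromBP, while NewMolecule fetches the molecule graph and appends an entry sized from its decode info.
; Helpers size and tag element spheres, create data-table-driven materials, find nearest atoms or visited neighbors, and spawn a molecule with attached Helium.
; Element-spawning chains in the event graph are disconnected.
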(event `self.ReceiveBeginPlay`
  (`self.SpawnObject` (0.0 0.0 -300.0) (struct) 2)
  (bind _returnvalue (`|CreateWidget` "/Game/Blueprints/buttonPlus.buttonPlus_C"))
  (`UserWidget.AddToViewport` _returnvalue 0))

(event `self.ReceiveTick`
  (params (DeltaSeconds :type "Float (single-precision)")))

(event `self.NewMolecule`
  (bind _tmp (`self.tmp`))
  (`KismetSystemLibrary.PrintString` "BP is activated")
  (`|ExecutionSequence`
    (:`then_0`
      (`self.GetMoleculeGraph`))
    (:`then_1`
      (bind _returnvalue (`self.GetMoleculeDecodeInfo`))
      (`KismetArrayLibrary.Array_Resize` _tmp (`KismetArrayLibrary.Array_Length` _returnvalue))
      (`KismetArrayLibrary.Array_Add` (`self.Molecules`) (make `Molecules` _tmp)))))

(event `/Game/Blueprints/inputInterface.OnTextCommitted`
  (params (input :type String))
  (if (`KismetStringLibrary.NotEqual_StrStr` input)
    (`self.SpawnGraphFromBP` input) ; Also Need to add check is input correct or not
  ))

(fn `CustomConstruction`
  (params (index :type Integer) (sphere :type "StaticMeshComponent Object Reference"))
  (returns (`dynamic material` :type "MaterialInstanceDynamic Object Reference"))
  (set `self.Tags` (`|MakeArray` (`KismetStringLibrary.Conv_StringToName` "element")))
  (bind _radius (`self.Get Atom Radius` index))
  (`SceneComponent.K2_AddLocalTransform` sphere (`KismetMathLibrary.MakeTransform` (0.0 0.0 0.0) (struct) (`KismetMathLibrary.Conv_DoubleToVector` _radius)) false false)
  (bind _material (`self.GetMaterial` index))
  (bind _returnvalue (`KismetMaterialLibrary.CreateDynamicMaterialInstance` _material))
  (return _returnvalue))

(fn `find closest`
  (params (ref :type "Actor Object Reference"))
  (returns (closest :type "Actor Object Reference"))
  (bind _outactors (`GameplayStatics.GetAllActorsWithTag` "element"))
  (set `self.closest actor` (`|GetArrayItem` _outactors))
  (for _array_element _outactors
    (if (!= _array_element ref)
      (if (< (`self.GetDistanceTo` _array_element ref) (`self.GetDistanceTo` (`self.closest actor`) ref))
        (set `self.closest actor` _array_element))))
  (return (`self.closest actor`)))

(fn `Find Previous`
  (params (neighbors :type "Array of Integer") (visited :type "Array of Boolean"))
  (returns (`Spawned Neighbor` :type Integer))
  (for _array_element neighbors
    (if (`|GetArrayItem` visited _array_element)
      (return _array_element))))

(fn `Get Atom Radius`
  (params (index :type Integer))
  (returns (radius :type "Float (double-precision)"))
  (if (`KismetMathLibrary.Conv_IntToBool` index)
    (bind _outrownames (`DataTableFunctionLibrary.GetDataTableRowNames` "/Game/Data/atomRadiusDataTable.atomRadiusDataTable"))
    (bind _returnvalue (`|GetDataTableRow` "/Game/Data/atomRadiusDataTable.atomRadiusDataTable" (`|GetArrayItem` _outrownames index))
      (:`then`
        (bind _output_get (set `self.AtomRadius` _returnvalue))
        (return (* (* (`.radius` (break `AtomRadius` _output_get)) (/ 1.0 29.0)) 0.5))))
    (else
      (`KismetSystemLibrary.PrintString` "No element with index 0" true true (struct :`R` 0.980208 :`G` 0.508742 :`B` 0.280052 :`A` 1.0)))))

(fn `GetMaterial`
  (params (index :type Integer))
  (returns (material :type "MaterialInterface Object Reference"))
  (if (`KismetMathLibrary.Conv_IntToBool` index)
    (bind _outrownames (`DataTableFunctionLibrary.GetDataTableRowNames` "/Game/Data/materialDataTable.materialDataTable"))
    (bind _returnvalue (`|GetDataTableRow` "/Game/Data/materialDataTable.materialDataTable" (`|GetArrayItem` _outrownames index))
      (:`then`
        (return (`.material_3_6473CCB9451E4CB10961C3B482D0ABB6` (break `/Game/Data/material` _returnvalue)))))
    (else
      (`KismetSystemLibrary.PrintString` "No element with index 0" true true (struct :`R` 0.980208 :`G` 0.508742 :`B` 0.280052 :`A` 1.0)))))

(fn `NewFunction_0`
  (`KismetSystemLibrary.PrintString` "NewFunction_0"))

(fn `Spawn molecule`
  (params (NewParam :type String))
  (locals (NewLocalVar_0 :type "Transform Structure"))
  (bind _returnvalue (`|SpawnActorFromClass` "/Game/Blueprints/Molecule2.Molecule2_C" (`self.GetTransform`) "Undefined" "OverrideRootScale" null NewParam null))
  (`|SpawnActorFromClass` "/Game/Blueprints/Helium.Helium_C" (`KismetMathLibrary.MakeTransform` (0.0 0.0 300.0)) "AlwaysSpawn" "OverrideRootScale" _returnvalue null)
  (bind _outactors (`GameplayStatics.GetAllActorsOfClass` "/Game/Blueprints/Helium.Helium_C"))
  (`self.K2_AttachToActor` (`|GetArrayItem` _outactors) _returnvalue "p1" "KeepRelative" "KeepRelative" "KeepRelative" true))

(fn `UserConstructionScript`)